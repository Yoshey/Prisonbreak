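; A breakable mesh that takes hits from damage or the screwdriver, then hides, loses collision and plays a break sound.
; Authority-side damage and the screwdriver's server overlap share one hit check that removes one Health per hit with a hit sound, regardless of damage amount.
; A DoOnce fires the break on the last hit.
; Round end restores visibility, collision and the Health saved in the construction script, and re-arms the DoOnce.
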(event `self.ReceiveBeginPlay`
  ;[1 0 0] Reset on Round Begin
  (`/Game/CustomMaps/UGC2095206091/PB/Miscellaneous/PrisonbreakFunctionLibrary.Event Round End` (delegate `Restart`)))

(event `resetall`
  (bind _staticmesh (`self.StaticMesh`))
  ;[1 0 0] Reset on Round Begin
  (`PrimitiveComponent.SetCollisionEnabled` _staticmesh "QueryAndPhysics")
  (`SceneComponent.SetVisibility` _staticmesh true false))

(event `soundforall`
  ;[1 0 1] Play Sound for All
  (`GameplayStatics.PlaySoundAtLocation` (`self.Hit Sound`) (`SceneComponent.K2_GetComponentLocation` (`self.StaticMesh`)) (struct) 1.0 1.0 0.0 "/Game/CustomMaps/UGC2095206091/PB/Miscellaneous/Sound/Attenuation/Normal.Normal" null null))

(event `Restart`
  ;[1 0 0] Reset on Round Begin
  (`|ExecutionSequence`
    (:`then_0`
      (`self.resetall`)
      (set `self.Health` (`self.HealthMemory`)))
    (:`then_1`
      (goto _label_2 :!via `Reset`))))

(event `self.Screwdriver_InteractBox.Screwdriver Overlap Client`
  (params (`Player Proxy` :type "/Game/CustomMaps/UGC2095206091/PB/Proxies/Prisonbreak_PlayerProxy Object Reference") (`Screwdriver Overlap Box` :type "/Game/CustomMaps/UGC2095206091/PB/Items/Prisoners/Screwdriver/Screwdriver_OverlapBox Object Reference") (Screwdriver :type "/Game/CustomMaps/UGC2095206091/PB/Items/Prisoners/Screwdriver/Screwdriver Object Reference"))
  ;[1 1 1] Start Overlapping
  (`/Game/CustomMaps/UGC2095206091/PB/Items/Prisoners/Screwdriver/Screwdriver.Cooldown` Screwdriver)
  (`/Game/CustomMaps/UGC2095206091/PB/Proxies/Prisonbreak_PlayerProxy.Replicate Screwdriver Overlap Server` `Player Proxy` `Screwdriver Overlap Box` Screwdriver))

(event `ServerHit`
  ;[0 1 0] Successful Hit
  (if (<= (`self.Health`) 1) :!label _label
    (`/Engine/EditorBlueprintResources/StandardMacros.DoOnce` false :!label _label_2
      (:`Completed`
        (`self.forall`)))
    (else
      (`/Engine/EditorBlueprintResources/StandardMacros.DecrementInt` (`self.Health`)
        (:`  `
          (`self.soundforall`))))))

(event `forall`
  (bind _staticmesh (`self.StaticMesh`))
  ;[1 1 1] Break wall
  (`PrimitiveComponent.SetCollisionEnabled` _staticmesh "NoCollision")
  (`SceneComponent.SetVisibility` _staticmesh false false)
  (`GameplayStatics.PlaySoundAtLocation` (`self.Break Sound`) (`SceneComponent.K2_GetComponentLocation` (`self.StaticMesh`)) (struct) 1.0 1.0 0.0 "/Game/CustomMaps/UGC2095206091/PB/Miscellaneous/Sound/Attenuation/Normal.Normal" null null))

(event `self.Screwdriver_InteractBox.Screwdriver Overlap Server`
  (params (Screwdriver :type "/Game/CustomMaps/UGC2095206091/PB/Items/Prisoners/Screwdriver/Screwdriver Object Reference"))
  ;[1 1 1] Start Overlapping Server
  (goto _label))

(event `self.ReceiveAnyDamage`
  (params (Damage :type "Float (single-precision)") (DamageType :type "DamageType Object Reference") (InstigatedBy :type "Controller Object Reference") (DamageCauser :type "Actor Object Reference"))
  ;[0 1 1] Shot?
  (`/Engine/EditorBlueprintResources/ActorMacros.Switch Has Authority`
    (:`Authority`
      (`self.ServerHit`))))

(fn `UserConstructionScript`
  (set `self.HealthMemory` (`self.Health`)))