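; Card-reader actor that spawns items, apparently knives, at two spawn points when an ID card touches it.
; The reader's overlap is forwarded to Runonserver, which accepts only IDCardcollider actors and passes them through a DoOnce gate.
; A valid swipe beeps, turns the reader red and calls SpawnItem on PrisonbreakGameLogic for each point.
; After a short delay the reader turns green and the gate resets for another swipe.
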(event `deactivatematerial`
  ;[1 1 1] Change Material Back
  (`PrimitiveComponent.SetMaterial` (`self.CardReaderMesh`) 1 "/Game/CustomMaps/UGC2095206091/PB/Miscellaneous/Materials/BasicColors/BasicGreen.BasicGreen"))

(event `activatesoundandmaterial`
  ;[1 1 1] Sound and Material Change
  (`GameplayStatics.PlaySoundAtLocation` "/Game/CustomMaps/UGC2095206091/PB/Miscellaneous/Sound/RadarBeep.RadarBeep" (`SceneComponent.K2_GetComponentLocation` (`self.CardReaderMesh`)) (struct) 1.0 1.0 0.0 "/Game/CustomMaps/UGC2095206091/PB/Miscellaneous/Sound/Attenuation/Normal.Normal" null null)
  (`PrimitiveComponent.SetMaterial` (`self.CardReaderMesh`) 1 "/Game/CustomMaps/UGC2095206091/PB/Miscellaneous/Materials/BasicColors/BasicRed.BasicRed"))

(event `runonserver`
  (params (`other actor` :type "Actor Object Reference"))
  (bind (_returnvalue_location _returnvalue_rotation) (`KismetMathLibrary.BreakTransform` (`SceneComponent.K2_GetComponentToWorld` (`self.knifespawn`))))
  (bind (_returnvalue_location_2 _returnvalue_rotation_2) (`KismetMathLibrary.BreakTransform` (`SceneComponent.K2_GetComponentToWorld` (`self.knifespawn2`))))
  ;[1 1 1] Execution
  (cast `/Game/CustomMaps/UGC2095206091/PB/Items/Guards/IDCard/IDCardcollider` `other actor`) ; Is an ID Card?
  (`/Engine/EditorBlueprintResources/StandardMacros.DoOnce` false :!label _label
    (:`Completed`
      (`self.activatesoundandmaterial`)
      (`|ExecutionSequence`
        (:`then_0`
          (`KismetSystemLibrary.Delay` 3.0)
          (`self.deactivatematerial`)
          (goto _label :!via `Reset`))
        (:`then_1`
          (bind _outactors (`GameplayStatics.GetAllActorsOfClass` "/Game/CustomMaps/UGC2095206091/PB/PrisonbreakGameLogic.PrisonbreakGameLogic_C"))
          (bind _output (`|GetArrayItem` _outactors))
          (`Pavlov_GameLogic.SpawnItem` _output (make `PavlovItemSpawnParams` "knife" null true false 0 true (`KismetMathLibrary.MakeTransform` _returnvalue_location _returnvalue_rotation)))
          (`Pavlov_GameLogic.SpawnItem` _output (make `PavlovItemSpawnParams` "knife" null true false 0 true (`KismetMathLibrary.MakeTransform` _returnvalue_location_2 _returnvalue_rotation_2))))))))

(event `self.cardreader.OnComponentBeginOverlap`
  (params (OverlappedComponent :type "PrimitiveComponent Object Reference") (OtherActor :type "Actor Object Reference") (OtherComp :type "PrimitiveComponent Object Reference") (OtherBodyIndex :type Integer) (bFromSweep :type Boolean) (SweepResult :type "HitResult Structure (by ref)"))
  ;[1 1 1] Run to Server
  (`self.runonserver` OtherActor))

(fn `UserConstructionScript`)