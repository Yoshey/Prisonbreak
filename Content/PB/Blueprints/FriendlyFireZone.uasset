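; Box trigger zone actor that marks pawns inside it with a "FriendlyFire" tag.
; The tag is added on begin overlap and removed on end overlap, with a Tick sweep of overlapping pawns as a fallback for any that missed it.
; RemoveTagsandDestroy sets a Stop flag to halt tagging, strips the tag from pawns still inside, then destroys the actor.
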(event `self.Box.OnComponentBeginOverlap`
  (params (OverlappedComponent :type "PrimitiveComponent Object Reference") (OtherActor :type "Actor Object Reference") (OtherComp :type "PrimitiveComponent Object Reference") (OtherBodyIndex :type Integer) (bFromSweep :type Boolean) (SweepResult :type "HitResult Structure (by ref)"))
  ;[1 1 1] Give Friendlyfire Tag when entering the Box
  (if (not (`self.Stop?`))
    (bind _aspawn (cast `Pawn` OtherActor))
    (`KismetArrayLibrary.Array_AddUnique` (`Actor.Tags` _aspawn) "FriendlyFire")))

(event `self.ReceiveTick`
  (params (DeltaSeconds :type "Float (single-precision)"))
  ;[1 1 1] Give Friendlyfire Tag when inside of the Box and it failed the first time
  (if (not (`self.Stop?`))
    (for _array_element (`PrimitiveComponent.GetOverlappingActors` (`self.Box`) "/Script/Engine.Pawn")
      (bind _tags (`Actor.Tags` _array_element))
      (if (not (`KismetArrayLibrary.Array_Contains` _tags "FriendlyFire"))
        (`KismetArrayLibrary.Array_AddUnique` _tags "FriendlyFire")))))

(event `self.Box.OnComponentEndOverlap`
  (params (OverlappedComponent :type "PrimitiveComponent Object Reference") (OtherActor :type "Actor Object Reference") (OtherComp :type "PrimitiveComponent Object Reference") (OtherBodyIndex :type Integer))
  ;[1 1 1] Remove FriendlyFire tag when leaving the Box
  (bind _aspawn (cast `Pawn` OtherActor))
  (`KismetArrayLibrary.Array_RemoveItem` (`Actor.Tags` _aspawn) "FriendlyFire"))

(event `Remove Tags and Destroy`
  ;[1 1 1] Remove Friendlyfire Tag from Prisoners in the Box and destroy the Box
  (set `self.Stop?` true)
  (for _array_element (`PrimitiveComponent.GetOverlappingActors` (`self.Box`) "/Script/Engine.Pawn")
    (`KismetArrayLibrary.Array_RemoveItem` (`Actor.Tags` _array_element) "FriendlyFire"))
  (`self.K2_DestroyActor`))

(fn `UserConstructionScript`)