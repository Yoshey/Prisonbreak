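; Example interactable for the Prisonbreak gamemode that fires a placeholder DoAction event when shot or used through its InteractBox.
; Client InteractBox events, including the wall-detection variant, forward the interaction to the server via InteractServer, whose server event then calls DoAction.
; Unwired sample branches show how to limit the action to guards or players with a special tag via GetPrisonbreakPlayerStatus.
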(event `self.ReceiveAnyDamage`
  (params (Damage :type "Float (single-precision)") (DamageType :type "DamageType Object Reference") (InstigatedBy :type "Controller Object Reference") (DamageCauser :type "Actor Object Reference"))
  ;[1 1 1] On overlap with InteractBox, check if actor is an Interactor. Then do an action.
  (`self.Do Action` :!label _label) ; Action for everyone
)

(event `self.Prisonbreak_InteractBox.OnInteractBoxClient`
  (params (InteractType :type "EInteractType Enum" :default "Grabbed") (HandProxy :type "Pavlov_HandProxy Object Reference") (InteractBox :type "Pavlov_InteractBox Object Reference"))
  ;[1 1 1] On overlap with InteractBox, check if actor is an Interactor. Then do an action.
  ;;[1 1 1] Send Interaction to Server
  (`Pavlov_InteractBox.InteractServer` (`self.Prisonbreak_InteractBox`) InteractType HandProxy InteractBox))

(event `self.Prisonbreak_InteractBox.OnInteractBoxServer`
  (params (InteractType :type "EInteractType Enum" :default "Grabbed") (HandProxy :type "Pavlov_HandProxy Object Reference") (InteractBox :type "Pavlov_InteractBox Object Reference"))
  ;[1 1 1] On overlap with InteractBox, check if actor is an Interactor. Then do an action.
  (goto _label))

(event `Do Action`
  ;[1 1 1] Do the thingy
)

(event `self.Prisonbreak_InteractBox.On Interact Box Client (Wall Detection)`
  (params (InteractType :type "EInteractType Enum" :default "Grabbed") (HandProxy :type "Pavlov_HandProxy Object Reference") (InteractObj :type "Object Object Reference"))
  ;[1 1 1] On overlap with InteractBox, check if actor is an Interactor. Then do an action.
  ;;[1 1 1] Only Send Interaction to Server if not reaching through a Wall
  (`Pavlov_InteractBox.InteractServer` (`self.Prisonbreak_InteractBox`) InteractType HandProxy InteractObj))

(fn `UserConstructionScript`)