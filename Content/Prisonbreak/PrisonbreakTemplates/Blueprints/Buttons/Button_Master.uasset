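; Base button for the Prisonbreak templates, pressed by shooting it or by player interaction.
; Damage on the authority and interact-box use, forwarded from the client to the server through the hand proxy, both fire ButtonGetsPressed, an empty hook here.
; Separate events swap activated and deactivated materials and play the press sound.
; Round end calls an empty RoundReset hook, and enabling also fires an empty hook.
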(event `Disable Button`
  ;[0 1 1] Change Material to Activate/Deactivate
  (`self.Change Button Material` (`self.Button Deactivated Material`)))

(event `Press Sound Multicast`
  ;[1 0 1] Play Sound Multicast
  (`GameplayStatics.PlaySoundAtLocation` (`self.Press Sound`) (`SceneComponent.K2_GetComponentLocation` (`self.ButtonMesh`)) (struct) 1.0 1.0 0.0 "/Game/Prisonbreak/PrisonbreakGamemode/Miscellaneous/Sound/Attenuation/Normal.Normal" null null))

(event `Change Button Material`
  (params (Material :type "MaterialInterface Object Reference"))
  ;[1 0 1] Change Material
  (`PrimitiveComponent.SetMaterial` (`self.ButtonMesh`) 0 Material))

(event `Enable Button`
  ;[0 1 1] Change Material to Activate/Deactivate
  (`self.Change Button Material` (`self.Button Activated Material`))
  (`self.Button gets Enabled`))

(event `Button gets Pressed`)

(event `self.ReceiveAnyDamage`
  (params (Damage :type "Float (single-precision)") (DamageType :type "DamageType Object Reference") (InstigatedBy :type "Controller Object Reference") (DamageCauser :type "Actor Object Reference"))
  ;[1 1 1] Execution
  (`/Engine/EditorBlueprintResources/ActorMacros.Switch Has Authority`
    (:`Authority`
      (`self.Button gets Pressed` :!label _label))))

(event `Round Reset`)

(event `self.Advanced_Interactbox.On Interact Box Client (Wall Detection)`
  (params (InteractType :type "EInteractType Enum" :default "Grabbed") (HandProxy :type "Pavlov_HandProxy Object Reference") (InteractObj :type "Object Object Reference"))
  ;[0 1 0] Player Interacts, tell Server
  (`Pavlov_HandProxy.ReplicateInteract_Server` HandProxy InteractType InteractObj))

(event `self.Advanced_Interactbox.OnInteractBoxServer`
  (params (InteractType :type "EInteractType Enum" :default "Grabbed") (HandProxy :type "Pavlov_HandProxy Object Reference") (InteractBox :type "Pavlov_InteractBox Object Reference"))
  ;[1 1 1] Execution
  (goto _label))

(event `Button gets Enabled`)

(event `Button is Pressed`
  ;[1 1 1] Button is Pressed
  (`self.Change Button Material` (`self.Button Deactivated Material`))
  (`self.Press Sound Multicast`))

(event `self.ReceiveBeginPlay`
  ;[1 0 0] Round End
  (`/Game/Prisonbreak/PrisonbreakGamemode/Miscellaneous/PrisonbreakFunctionLibrary.Event Round End` (delegate `Round End`)))

(event `Round End`
  ;[1 0 0] Round End
  (`self.Round Reset`))

(fn `UserConstructionScript`)