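; ID card scanner that slides a target door open and closed with a timeline, sounds and scanner material feedback.
; Card overlaps relay through the player proxy to the server, where a DoOnce throttles scans and fires a multicast toggle, with optional delayed auto-close.
; Scanners sharing a door route to one Primary, found in the construction script, so door state stays in one place.
; Round end resets the timeline and open state.
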(event `self.IDCard_OverlapBox.Developer Mode`
  ;[1 1 1] Developer Mode
  (`/Engine/EditorBlueprintResources/ActorMacros.Switch Has Authority`
    (:`Authority`
      (bind _enabled_ (`/Game/Prisonbreak/PrisonbreakGamemode/Miscellaneous/PrisonbreakFunctionLibrary.Developer Mode?`))
      (if _enabled_
        ;[1 1 1] Execution
        (`/Engine/EditorBlueprintResources/StandardMacros.DoOnce` false :!label _label
          (:`Completed`
            (`self.activatesoundandmaterial`)
            (`|ExecutionSequence`
              (:`then_0`
                (`KismetSystemLibrary.Delay` (`self.Delay Before Button Resets`))
                (`self.deactivatematerial`)
                (goto _label :!via `Reset`))
              (:`then_1`
                (`self.Multicast` (`self.Primary`))
                (`self.Automatic Close`)))))))))

(event `activatesoundandmaterial`
  ;[1 0 1] Sound and Material Change
  (`GameplayStatics.PlaySoundAtLocation` (`self.Scan Sound`) (`SceneComponent.K2_GetComponentLocation` (`self.CardReaderMesh`)) (struct) 1.0 1.0 0.0 "/Game/Prisonbreak/PrisonbreakGamemode/Miscellaneous/Sound/Attenuation/Normal.Normal" null null)
  (`PrimitiveComponent.SetMaterial` (`self.CardReaderMesh`) 1 (`self.Scanner Activated`)))

(event `deactivatematerial`
  ;[1 0 1] Change Material Back
  (`PrimitiveComponent.SetMaterial` (`self.CardReaderMesh`) 1 (`self.Scanner Deactivated`)))

(event `self.IDCard_OverlapBox.IDCard Overlap Client`
  (params (`Player Proxy` :type "/Game/Prisonbreak/PrisonbreakGamemode/Proxies/Prisonbreak_PlayerProxy Object Reference") (`IDCard Overlap Box` :type "/Game/Prisonbreak/PrisonbreakGamemode/Items/Guards/IDCard/IDCard_OverlapBox Object Reference") (IDCard :type "/Game/Prisonbreak/PrisonbreakGamemode/Items/Guards/IDCard/IDCard Object Reference"))
  ;[1 1 1] Replicate Client interaction to Server
  (`/Game/Prisonbreak/PrisonbreakGamemode/Proxies/Prisonbreak_PlayerProxy.Replicate IDCard Overlap Server` `Player Proxy` `IDCard Overlap Box` IDCard))

(event `self.IDCard_OverlapBox.IDCard Overlap Server`
  (params (IDCard :type "/Game/Prisonbreak/PrisonbreakGamemode/Items/Guards/IDCard/IDCard Object Reference"))
  ;[1 1 1] Execution
  (goto _label))

(event `self.ReceiveBeginPlay`
  ;[1 0 0] Round End
  (`/Game/Prisonbreak/PrisonbreakGamemode/Miscellaneous/PrisonbreakFunctionLibrary.Event Round End` (delegate `Round End`)))

(event `Multicast`
  (bind _door_location (`self.Door Location`))
  (bind (_door_location_x _door_location_y _door_location_z) (`KismetMathLibrary.BreakVector` (`self.Door Location`)))
  ;[0 1 0] Door Logic Smooth
  (if (`self.Open?`)
    (if (not (`self.Retrigger to Reset Timer?`))
      (`GameplayStatics.PlaySoundAtLocation` (`self.Close Sound`) _door_location (struct) 1.0 1.0 0.0 "/Game/Prisonbreak/PrisonbreakGamemode/Miscellaneous/Sound/Attenuation/Normal.Normal" null null :!label _label_2)
      (set `self.Open?` false)
      (bind (_direction _newtrack_0) (`Timeline|Open/Close` :!via `Reverse` :!label _label_3)
        (:`Update`
          (bind (_x _y _z) (`/Game/Prisonbreak/PrisonbreakGamemode/Miscellaneous/PrisonbreakMacroLibrary.Smooth Direction Logic` _newtrack_0 (`self.Distance`) _door_location_x _door_location_y _door_location_z (`self.Direction Up/Down`) (`self.Direction Left/Right`) (`self.Flip Left/Right with Forwards/Backwards`)))
          (`SceneComponent.K2_SetWorldLocation` (`Actor.RootComponent` (`self.Target Door`)) (`KismetMathLibrary.MakeVector` _x _y _z) false false))))
    (else
      (`GameplayStatics.PlaySoundAtLocation` (`self.Open Sound`) _door_location (struct) 1.0 1.0 0.0 "/Game/Prisonbreak/PrisonbreakGamemode/Miscellaneous/Sound/Attenuation/Normal.Normal" null null)
      (set `self.Open?` true)
      (goto _label_3))))

(event `Round End`
  ;[1 0 0] Round End
  (`self.Reset Animation`))

(event `Close Door`
  ;[0 1 0] Door Logic Smooth
  (if (`self.Open?`)
    (goto _label_2)))

(event `Reset Animation`
  ;[1 0 0] Reset Animation
  (`|ExecutionSequence`
    (:`then_0`
      (goto _label_3 :!via `Stop`))
    (:`then_1`
      (goto _label_3 :!via `SetNewTime`))
    (:`then_2`
      (set `self.Open?` false))))

(event `Automatic Close`
  ;[1 1 1] Automatic Close
  (if (`self.Close Automatically?`)
    (`KismetSystemLibrary.RetriggerableDelay` (`self.Delay before Automatic Close`))
    (`self.Close Door` (`self.Primary`))))

(fn `UserConstructionScript`
  (`TimelineComponent.SetPlayRate` (`self.Open/Close`) (`self.Speed`))
  (`/Engine/EditorBlueprintResources/ActorMacros.Switch Has Authority`
    (:`Authority`
      (set `self.Door Location` (`self.K2_GetActorLocation` (`self.Target Door`)))
      (bind (_direction_up_down _direction_left_right) (`/Game/Prisonbreak/PrisonbreakGamemode/Miscellaneous/PrisonbreakFunctionLibrary.Up/Down/Left/Right Direction Setting` (`self.Up`) (`self.Down`) (`self.Left`) (`self.Right`)))
      (set `self.Direction Up/Down` _direction_up_down)
      (set `self.Direction Left/Right` _direction_left_right)
      (bind _outactors (`GameplayStatics.GetAllActorsOfClass` "IDCardScannerDoor_Smooth_C"))
      (for _array_element _outactors
        (if (== (`self.Target Door`) (`/Game/Prisonbreak/PrisonbreakTemplates/Blueprints/IDCardScanners/IDCardScannerDoor_Smooth.Target Door` _array_element))
          (set `self.Primary` _array_element)
          (break))))))