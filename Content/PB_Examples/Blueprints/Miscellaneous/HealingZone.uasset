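; Example Pavlov healing zone that restores health to pawns inside its Box volume.
; BeginPlay calls a Server event that loops every second over overlapping pawns and reads their Pavlov player status.
; Pawns at or below 100 health are healed through negative ApplyDamage.
; Above 100 it calls a small positive ApplyDamage, but that call has no target actor wired.
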(event `server`
  (for _array_element (`PrimitiveComponent.GetOverlappingActors` (`self.Box`) "/Script/Engine.Pawn") :!label _label
    (bind _aspawn (cast `Pawn` _array_element))
    (bind _playerstatus (`PavlovProxyStatics.GetPavlovPlayerStatusByPawn` _aspawn))
    (bind (_playerstate _controller _pawn _steamid _cash _score _teamid _health) (break `PavlovPlayerStatus` _playerstatus))
    (if (> _health 100)
      (if (not (== _health 100))
        (`GameplayStatics.ApplyDamage` null 1.0))
      (else
        (`GameplayStatics.ApplyDamage` _aspawn -10.0))))
  (`KismetSystemLibrary.Delay` 1.0)
  (goto _label))

(event `self.ReceiveBeginPlay`
  (`self.server`))

(fn `UserConstructionScript`)