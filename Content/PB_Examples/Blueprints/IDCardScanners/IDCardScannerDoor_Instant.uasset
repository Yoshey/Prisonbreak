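; An ID card scanner that instantly toggles a target door between hidden and visible.
; A client card overlap is relayed to the server through the player proxy, then plays a scan sound and swaps the reader material, with a timed DoOnce reset.
; The door toggle keys off its collision state through multicast events, with optional retriggerable automatic closing.
; Round end makes the door visible again.
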(event `activatesoundandmaterial`
  ;[1 0 1] Sound and Material Change
  (`GameplayStatics.PlaySoundAtLocation` (`self.Scan Sound`) (`SceneComponent.K2_GetComponentLocation` (`self.CardReaderMesh`)) (struct) 1.0 1.0 0.0 "/Game/PB/Miscellaneous/Sound/Attenuation/Normal.Normal" null null)
  (`PrimitiveComponent.SetMaterial` (`self.CardReaderMesh`) 1 (`self.Scanner Activated`)))

(event `deactivatematerial`
  ;[1 0 1] Change Material Back
  (`PrimitiveComponent.SetMaterial` (`self.CardReaderMesh`) 1 (`self.Scanner Deactivated`)))

(event `self.IDCard_OverlapBox.IDCard Overlap Client`
  (params (`Player Proxy` :type "/Game/PB/Proxies/Prisonbreak_PlayerProxy Object Reference") (`IDCard Overlap Box` :type "/Game/PB/Items/Guards/IDCard/IDCard_OverlapBox Object Reference") (IDCard :type "/Game/PB/Items/Guards/IDCard/IDCard Object Reference"))
  ;[1 1 1] IDCard Overlap
  (`/Game/PB/Proxies/Prisonbreak_PlayerProxy.Replicate IDCard Overlap Server` `Player Proxy` `IDCard Overlap Box` IDCard))

(event `self.IDCard_OverlapBox.IDCard Overlap Server`
  (params (IDCard :type "/Game/PB/Items/Guards/IDCard/IDCard Object Reference"))
  ;[1 1 1] Execution
  (`/Engine/EditorBlueprintResources/StandardMacros.DoOnce` false :!label _label
    (:`Completed`
      (`self.activatesoundandmaterial`)
      (`|ExecutionSequence`
        (:`then_0`
          (`KismetSystemLibrary.Delay` (`self.Time before Button Resets`))
          (`self.deactivatematerial`)
          (goto _label :!via `Reset`))
        (:`then_1`
          (`self.Multicast`))))))

(event `self.ReceiveBeginPlay`
  ;[1 0 0] Round End
  (`/Game/PB/Miscellaneous/PrisonbreakFunctionLibrary.Event Round End` (delegate `Round End`)))

(event `Multicast`
  (bind _target_door (`self.Target Door`))
  ;[0 1 0] Door Logic Instant
  (if (`self.GetActorEnableCollision` (`self.Target Door`))
    (`/Game/PB/Miscellaneous/PrisonbreakMacroLibrary.Make Door Invisible` _target_door
      (:`Out`
        (`self.Multicast Automatic Close`)))
    (else
      (`/Game/PB/Miscellaneous/PrisonbreakMacroLibrary.Make Door Visible` _target_door :!label _label_2))))

(event `Round End`
  ;[1 0 0] Round End
  (`self.Multicast Visible`))

(event `Multicast Visible`
  ;[0 1 0] Door Logic Instant
  (goto _label_2))

(event `Multicast Automatic Close`
  ;[1 1 1] Automatic Close
  (if (`self.Close Automatically?`)
    (`KismetSystemLibrary.RetriggerableDelay` (`self.Delay before Automatic Close`))
    (if (not (`self.GetActorEnableCollision` (`self.Target Door`)))
      (`/Game/PB/Miscellaneous/PrisonbreakMacroLibrary.Make Door Visible` (`self.Target Door`)))))

(fn `UserConstructionScript`
  (`/Engine/EditorBlueprintResources/ActorMacros.Switch Has Authority`
    (:`Authority`
      (set `self.Door Location` (`self.K2_GetActorLocation` (`self.Target Door`))))))