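; Prison Break button that opens every Celldoor in the level when damaged, interacted with or timed out, and unmutes everyone via the game logic.
; A server DoOnce fires a multicast that hides the button, plays a sound and slides doors by timeline along construction-set directions, then disables their collision.
; Preround resets restore button and collision and restart the server's auto-open countdown, or trigger opening immediately when the one-player check passes.
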(event `Timer Up`
  ;[0 1 0] Execution on Server
  (`/Engine/EditorBlueprintResources/StandardMacros.DoOnce` false :!label _label
    (:`Completed`
      (set `self.reset?` false)
      (set `self.timer` 120)
      (`self.Multicast`)
      (bind _asprisonbreak_game_logic (cast `/Game/PB/PrisonbreakGameLogic` (`Pavlov_Library.GetGameLogic`)))
      (`/Game/PB/PrisonbreakGameLogic.Unmute Everyone` _asprisonbreak_game_logic))))

(event `self.ReceiveAnyDamage`
  (params (Damage :type "Float (single-precision)") (DamageType :type "DamageType Object Reference") (InstigatedBy :type "Controller Object Reference") (DamageCauser :type "Actor Object Reference"))
  ;[0 1 0] Execution on Server
  (goto _label))

(event `Multicast`
  (bind _returnvalue (* (`self.Mover`) (`self.Distance`)))
  ;[0 1 0] Execution on All
  (`SceneComponent.SetVisibility` (`self.StaticMesh`) false false)
  (`GameplayStatics.PlaySound2D` (`self.Cell Open Sound`) 1.0 1.0 0.0 null null)
  (bind (_direction _newtrack_0) (`Timeline|Open` :!via `PlayFromStart` :!label _label_2)
    (:`Update`
      (set `self.Mover` _newtrack_0)
      (for _array_element (`self.Cell Doors`)
        (`SceneComponent.K2_SetRelativeLocation` (`/Game/PB_Examples/Blueprints/Cells/Celldoor.Doormesh` _array_element) (`KismetMathLibrary.MakeVector` 0.0 (select `int` (`self.Direction Left/Right`) :`0` _returnvalue :`1` 0.0 :`2` (* _returnvalue -1.0)) (select `int` (`self.Direction Up/Down`) :`0` _returnvalue :`1` 0.0 :`2` (* _returnvalue -1.0))) false false)))
    (:`Finished`
      (if (not (`self.reset?`))
        (for _array_element_2 _
          (`PrimitiveComponent.SetCollisionEnabled` (`/Game/PB_Examples/Blueprints/Cells/Celldoor.Doormesh` _array_element_2) "NoCollision"))))))

(event `self.Advanced_Interactbox.OnInteractBoxServer`
  (params (InteractType :type "EInteractType Enum" :default "Grabbed") (HandProxy :type "Pavlov_HandProxy Object Reference") (InteractBox :type "Pavlov_InteractBox Object Reference"))
  ;[0 1 0] Execution on Server
  (goto _label))

(event `Reset Movement`
  ;[0 1 0] Execution on All
  (`|ExecutionSequence`
    (:`then_0`
      (goto _label_2 :!via `Stop`))
    (:`then_1`
      (goto _label_2 :!via `SetNewTime`))))

(event `self.ReceiveBeginPlay`
  ;[1 0 0] Reset on Round End
  (bind _outactors (`GameplayStatics.GetAllActorsOfClass` "/Game/PB/PrisonbreakGameLogic.PrisonbreakGameLogic_C"))
  (add `/Game/PB/PrisonbreakGameLogic.Preround Dispatcher` (`|GetArrayItem` _outactors) (delegate `reset round begin`)))

(event `Reset Cells Multicast`
  ;[1 1 1] Reset Cells at round Restart
  (`SceneComponent.SetVisibility` (`self.StaticMesh`) true false)
  (`|ExecutionSequence`
    (:`then_0`
      (set `self.reset?` true)
      (`self.Reset Movement`))
    (:`then_1`
      (for _array_element (`self.Cell Doors`)
        (`PrimitiveComponent.SetCollisionEnabled` (`/Game/PB_Examples/Blueprints/Cells/Celldoor.Doormesh` _array_element) "QueryAndPhysics"))
      (`/Engine/EditorBlueprintResources/ActorMacros.Switch Has Authority`
        (:`Authority`
          (set `self.timer` 0)
          (`|ExecutionSequence`
            (:`then_0`
              (`KismetSystemLibrary.Delay` 2.0)
              (goto _label :!via `Reset`))
            (:`then_1`
              ;;[0 1 1] Open Cells Automatically after 2 Minutes
              (bind _result (`/Engine/EditorBlueprintResources/StandardMacros.IncrementInt` (`self.timer`) :!label _label_3)
                (:`  `
                  (if (>= _result (`self.Open Cells Automatically`))
                    (`self.Timer Up`)
                    (else
                      (`KismetSystemLibrary.Delay` 1.0)
                      (goto _label_3))))))))))))

(event `reset round begin`
  ;[1 0 0] Reset on Round End
  (`self.reset`))

(event `reset`
  ;[1 1 1] Reset Cells at round Restart
  (`/Game/PB/Miscellaneous/PrisonbreakMacroLibrary.1 Player is Enough to Start?`
    (:`Yes`
      (`self.Timer Up`))
    (:`No`
      (`self.Reset Cells Multicast`))))

(fn `UserConstructionScript`
  (`TimelineComponent.SetPlayRate` (`self.Open`) (`self.Speed`))
  (bind _outactors (`GameplayStatics.GetAllActorsOfClass` "/Game/PB_Examples/Blueprints/Cells/Celldoor.Celldoor_C"))
  (set `self.Cell Doors` _outactors)
  (`|ExecutionSequence`
    (:`then_0`
      (if (`self.Up`)
        (if (`self.Down`)
          (set `self.Direction Up/Down` 1 :!label _label)
          (else
            (set `self.Direction Up/Down` 2)))
        (elif (`self.Down`)
          (set `self.Direction Up/Down` 0)
          (else
            (goto _label)))))
    (:`then_1`
      (if (`self.Left`)
        (if (`self.Right`)
          (set `self.Direction Left/Right` 1 :!label _label_2)
          (else
            (set `self.Direction Left/Right` 2)))
        (elif (`self.Right`)
          (set `self.Direction Left/Right` 0)
          (else
            (goto _label_2)))))))